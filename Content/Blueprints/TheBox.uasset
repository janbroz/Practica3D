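; TheBox is an actor that moves its PMesh forward by Speed every tick, without sweep or delta-time scaling, and can explode.
; Construction and BeginPlay both copy NewSize into Size.
; KillItwithFire destroys it with an explosion effect and a sound played at world origin.
; TimeToDie also awards score to PracticaPlayerController and plays the sound at the box, but its timer setup is unconnected.
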(event EventBeginPlay
  (Variables|Default|SetSize (Variables|Default|GetNewSize)))

(event Collision|EventActorBeginOverlap
  (params (OtherActor :type Actor%20Object%20Reference)))

(event EventTick
  (params (DeltaSeconds :type Float%20%28single-precision%29))
  (bind _p_mesh (Variables|Default|GetP_mesh))
  (Transformation|SetWorldLocation _p_mesh (+ (Transformation|GetWorldLocation _p_mesh) (* (Math|Vector|GetForwardVector _p_mesh) (Variables|Default|GetSpeed))) false false))

(event EventKillItwithFire
  (Effects|SpawnEmitteratLocation "/Game/StarterContent/Particles/P_Explosion.P_Explosion" (Transformation|GetActorLocation))
  (Audio|PlaySoundatLocation "/Game/StarterContent/Audio/Explosion01.Explosion01" "0, 0, 0")
  (Actor|DestroyActor))

(fn ConstructionScript
  (Variables|Default|SetSize (Variables|Default|GetNewSize)))

(fn TimetoDie
  (bind _returnvalue (Transformation|GetActorLocation))
  (bind _aspractica_player_controller (Utilities|Casting|CastToPracticaPlayerController (Game|GetPlayerController 0)))
  (Variables|/Script/Practica3D.PracticaPlayerController|SetScore _aspractica_player_controller (+ (Variables|/Script/Practica3D.PracticaPlayerController|GetScore _aspractica_player_controller) 10))
  (Effects|SpawnEmitteratLocation "/Game/StarterContent/Particles/P_Explosion.P_Explosion" _returnvalue)
  (Audio|PlaySoundatLocation "/Game/StarterContent/Audio/Explosion01.Explosion01" _returnvalue)
  (Actor|DestroyActor))