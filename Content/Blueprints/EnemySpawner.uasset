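; Enemy spawner actor that periodically spawns evil boxes of a configurable class.
; BeginPlay starts a looping timer at SpawnRate that calls SpawnEvilBox.
; Each spawn copies the spawner's transform with a random offset along world Y and passes the new box a random Speed through an exposed spawn parameter.
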(event EventBeginPlay
  (Utilities|Time|SetTimerbyFunctionName 0 "SpawnEvilBox" (Variables|Default|GetSpawnRate) true))

(event Collision|EventActorBeginOverlap
  (params (OtherActor :type Actor%20Object%20Reference)))

(event EventTick
  (params (DeltaSeconds :type Float%20%28single-precision%29)))

(fn ConstructionScript)

(fn SpawnEvilBox
  (bind _returnvalue (Transformation|GetActorTransform))
  (bind (_location _rotation _scale) (Math|Transform|BreakTransform _returnvalue))
  (bind (_x _y _z) (Math|Vector|BreakVector _location))
  ;[1 1 1] Spawn the black, spawn the black box!
  (Game|SpawnActorfromClass (Variables|Default|GetBoxClass) (Math|Transform|MakeTransform (Math|Vector|MakeVector _x (+ _y (Math|Random|RandomFloatinRange -5e+02 5e+02)) _z) _rotation _scale) "Undefined" 0 (Math|Random|RandomFloatinRange 1.0 5.0) 1e+02 0))